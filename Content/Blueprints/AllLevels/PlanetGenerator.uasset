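; PlanetGenerator is a planet actor that randomly rescales itself during play and provides a spherical surface query.
; Tick passes through a one-second Delay, prints a random vector, then sets Sphere and Planet to a separately randomized per-axis scale at the Sphere's location with zero rotation.
; The random unit-vector checks before the transform always pass, as their threshold is unreachable.
; GetSurfaceLocationAndNormalAt projects a location onto the RadiusinUnits sphere around the actor.
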(event EventTick
  (params (DeltaSeconds :type Float%20%28single-precision%29))
  (bind _returnvalue (Math|Random|RandomUnitVector))
  (bind _returnvalue_2 (Math|Random|RandomFloatinRange 1e+01 2e+01))
  (bind _returnvalue_3 (Math|Vector|MakeVector _returnvalue_2 _returnvalue_2 _returnvalue_2))
  (bind _returnvalue_4 (* _returnvalue "10.000000,10.000000,10.000000"))
  (bind (_x _y _z) (Math|Vector|BreakVector _returnvalue_4))
  (Utilities|FlowControl|Delay 1.0)
  (Development|PrintString (Utilities|String|ToString(Vector) _returnvalue_3))
  (if (not (>= _x 1e+02))
    (if (not (>= _y 1e+02))
      (if (not (>= _z 1e+02))
        (Transformation|SetWorldTransform (Variables|Default|GetSphere) (Math|Transform|MakeTransform (Transformation|GetWorldLocation (Variables|Default|GetSphere)) "0, 0, 0" _returnvalue_3) false false)))))

(fn ConstructionScript)

(fn GetSurfaceLocationandNormalat
  (params (Location :type Vector))
  (bind _returnvalue (Transformation|GetActorLocation))
  (bind _returnvalue_2 (- Location _returnvalue))
  (bind _returnvalue_3 (Math|Vector|Normalize _returnvalue_2))
  (return (+ (* _returnvalue_3 (Variables|Default|GetRadiusinUnits)) (Transformation|GetActorLocation)) _returnvalue_3))