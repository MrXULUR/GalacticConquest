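; Main character controller that lets the player press E to switch possession between the first-person character and a TurboLaser turret.
; Entering requires overlapping the turret's box and destroys the character; exiting spawns a new one offset above the turret camera.
; Tick binds the overlap events and checks the possessed pawn's class.
; Paired DoOnce gates re-arm each other, IsAiReady flags on-foot state, and actor references refresh after each press.
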(event Custom|Reset-1
  ;[1 1 1] Character Possession Code, and yah it is fucking to long . . . BUT IT WORKS
  (Utilities|FlowControl|DoOnce false) ; enters at Reset
)

(event Custom|OnComponentEndOverlap_Event
  (params (OverlappedComponent :type Primitive%20Component%20Object%20Reference) (OtherActor :type Actor%20Object%20Reference) (OtherComp :type Primitive%20Component%20Object%20Reference) (OtherBodyIndex :type Integer))
  ;[1 1 1] Character Possession Code, and yah it is fucking to long . . . BUT IT WORKS
  (Variables|Default|SetOverlap%20Bool false)
  (Development|PrintString "NOT"))

(event Custom|Reset-2
  ;[1 1 1] Character Possession Code, and yah it is fucking to long . . . BUT IT WORKS
  (Utilities|FlowControl|DoOnce false) ; enters at Reset
)

(event Custom|OnComponentBeginOverlap_Event
  (params (OverlappedComponent :type Primitive%20Component%20Object%20Reference) (OtherActor :type Actor%20Object%20Reference) (OtherComp :type Primitive%20Component%20Object%20Reference) (OtherBodyIndex :type Integer) (bFromSweep :type Boolean) (SweepResult :type Hit%20Result%20Structure%20%28by%20ref%29))
  ;[1 1 1] Character Possession Code, and yah it is fucking to long . . . BUT IT WORKS
  (Utilities|Casting|CastToFirstPersonCharacter OtherActor)
  (Variables|Default|SetOverlap%20Bool true)
  (Development|PrintString "Overlapped"))

(event EventBeginPlay
  ;[1 1 1] Character Possession Code, and yah it is fucking to long . . . BUT IT WORKS
  (Variables|Default|SetIs%20AiReady true)
  (Utilities|FlowControl|Sequence
    (:then_0
      (bind _outactors (Actor|GetAllActorsOfClass "/Game/Blueprints/TurboLaser.TurboLaser_C"))
      (for _array_element _outactors
        (Variables|Default|SetTurboLaser _array_element)
        (bind _outactors_2 (Actor|GetAllActorsOfClass "/Game/FirstPersonBP/Blueprints/FirstPersonCharacter.FirstPersonCharacter_C"))
        (for _array_element_2 _outactors_2
          (Variables|Default|SetFirstPersonCharacter _array_element_2))))))

(event EventTick
  (params (DeltaSeconds :type Float%20%28single-precision%29))
  (bind _returnvalue (Pawn|GetControlledPawn))
  (bind _turbolaser (Variables|Default|GetTurboLaser))
  (bind _returnvalue_2 (Utilities|GetClass _returnvalue))
  (bind _box (Variables|/Game/Blueprints/TurboLaser.TurboLaser_C|GetBox _turbolaser))
  ;[1 1 1] Character Possession Code, and yah it is fucking to long . . . BUT IT WORKS
  (Utilities|FlowControl|Sequence
    (:then_0
      (Collision|BindEventtoOnComponentBeginOverlap _box (delegate Custom|OnComponentBeginOverlap_Event))
      (Variables|Default|SetIs%20TurboLaser (== _returnvalue_2 "/Game/Blueprints/TurboLaser.TurboLaser_C"))
      (Variables|Default|SetIs%20Character (== _returnvalue_2 "/Game/FirstPersonBP/Blueprints/FirstPersonCharacter.FirstPersonCharacter_C")))
    (:then_1
      (Collision|BindEventtoOnComponentEndOverlap _box (delegate Custom|OnComponentEndOverlap_Event)))))

(event Input|KeyboardEvents|E
  (params (Key :type Key%20Structure))
  ;[1 1 1] Character Possession Code, and yah it is fucking to long . . . BUT IT WORKS
  (:Pressed
    (Utilities|FlowControl|Sequence
      (:then_0
        (if (Variables|Default|GetIs%20Character)
          (if (Variables|Default|GetOverlap%20Bool)
            (Utilities|FlowControl|DoOnce false
              (:Completed
                (Pawn|Possess (Game|GetPlayerController 0) (Variables|Default|GetTurboLaser))
                (Actor|DestroyActor (Variables|Default|GetFirstPersonCharacter))
                (Variables|Default|SetIs%20AiReady false)
                (CallFunction|Reset-1))))))
      (:then_1
        (if (Variables|Default|GetIs%20TurboLaser)
          (Utilities|FlowControl|DoOnce false
            (:Completed
              (bind _returnvalue (Game|SpawnActorfromClass "/Game/FirstPersonBP/Blueprints/FirstPersonCharacter.FirstPersonCharacter_C" (Math|Transform|MakeTransform (+ (.Location (Math|Transform|BreakTransform (Transformation|GetWorldTransform (Variables|/Game/Blueprints/TurboLaser.TurboLaser_C|GetCamera (Variables|Default|GetTurboLaser))))) "100.000000, 0,1000.000000")) "Undefined" 0 0))
              (Pawn|Possess (Game|GetPlayerController 0) _returnvalue)
              (Variables|Default|SetIs%20AiReady true)
              (CallFunction|Reset-2)))))
      (:then_2
        (Utilities|FlowControl|Sequence
          (:then_0
            (bind _outactors (Actor|GetAllActorsOfClass "/Game/Blueprints/TurboLaser.TurboLaser_C"))
            (for _array_element _outactors
              (Variables|Default|SetTurboLaser _array_element)
              (bind _outactors_2 (Actor|GetAllActorsOfClass "/Game/FirstPersonBP/Blueprints/FirstPersonCharacter.FirstPersonCharacter_C"))
              (for _array_element_2 _outactors_2
                (Variables|Default|SetFirstPersonCharacter _array_element_2)))))))))

(fn ConstructionScript)