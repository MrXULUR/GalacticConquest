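; TurretAiController steers the barrel of a TurboLaser turret toward the player pawn.
; On BeginPlay it finds TurboLaser and MainCharacterController actors by class, keeping only the last of each.
; While the controller's IsAiReady flag is false, Tick smoothly turns the barrel with RInterpTo, yaw only, using a look-at rotation offset by a quarter turn.
; When the flag is true, it only prints the value and the barrel stays still.
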(event EventTick
  (params (DeltaSeconds :type Float%20%28single-precision%29))
  (bind _maincontroller (Variables|Default|GetMainController))
  (bind _is_aiready (Variables|/Game/Blueprints/MainCharacterController.MainCharacterController_C|GetIs%20AiReady _maincontroller))
  (Variables|Default|SetDeltaTime DeltaSeconds)
  (if _is_aiready
    (Development|PrintString (Utilities|String|ToString(Boolean) _is_aiready))
    (else
      (Transformation|SetWorldRotation (Variables|/Game/Blueprints/TurboLaser.TurboLaser_C|GetBarrel (Variables|Default|GetTurboLaser)) (Math|Interpolation|RInterpTo (Transformation|GetWorldRotation (Variables|/Game/Blueprints/TurboLaser.TurboLaser_C|GetBarrel (Variables|Default|GetTurboLaser))) (Math|Rotator|MakeRotator 0.0 0.0 (- (.Yaw (Math|Rotator|BreakRotator (Math|Rotator|FindLookatRotation (Transformation|GetWorldLocation (Variables|/Game/Blueprints/TurboLaser.TurboLaser_C|GetBarrel (Variables|Default|GetTurboLaser))) (Transformation|GetActorLocation (Game|Player|GetPlayerPawn 0))))) 9e+01)) (Variables|Default|GetDeltaTime) (Variables|Default|GetRotationSpeed)) false false))))

(event EventBeginPlay
  (bind _outactors (Actor|GetAllActorsOfClass "/Game/Blueprints/TurboLaser.TurboLaser_C"))
  (for _array_element _outactors
    (Variables|Default|SetTurboLaser _array_element)
    (bind _outactors_2 (Actor|GetAllActorsOfClass "/Game/Blueprints/MainCharacterController.MainCharacterController_C"))
    (for _array_element_2 _outactors_2
      (Variables|Default|SetMainController _array_element_2))))

(fn ConstructionScript)