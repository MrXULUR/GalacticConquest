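; AI controller for TurboLaser turrets, meant to aim at the player and fire, but all its events are empty and the logic is left unwired.
; The disconnected nodes would cache the turret and MainCharacterController, then run a behavior tree on possession.
; They also hold interpolated arrow rotation toward the player, gated by IsAiReady, and a range-based AiFire call.
; The perception handler's disconnected logic only casts to Character_Base.
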(event OnTargetPerceptionUpdated(AIPerception)
  (params (Actor :type Actor%20Object%20Reference) (Stimulus :type AI%20Stimulus%20Structure)))

(event Custom|AimAt
  (params (DeltaTime :type Float%20%28single-precision%29))
  ;[1 1 1] BECAUSE THINGS CAN'T BE SIMPLE!
)

(event Custom|AiFire
  ;[1 1 1] AiFireAt
)

(event EventOnPossess
  (params (PossessedPawn :type Pawn%20Object%20Reference)))

(event EventTick
  (params (DeltaSeconds :type Float%20%28single-precision%29))
  ;[1 1 1] Tick Events
)

(event EventBeginPlay
  ;[1 1 1] AiControl
)

(fn ConstructionScript)