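; Controller Blueprint that lets the player swap between walking as Character_Base and manning a TurboLaser with E.
; BeginPlay and each E press cache the actors found in the level; Tick checks the pawn class and binds the character's sphere overlaps.
; E during overlap possesses the turret and destroys the character; E again spawns and possesses a new one offset from the turret camera.
; Paired DoOnce gates reset each other; capture zone logic is unfinished.
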(event Custom|Reset-1
  ;[1 1 1] Character Possession Code, and yah it is fucking to long . . . BUT IT WORKS
  (Utilities|FlowControl|DoOnce false) ; enters at Reset
)

(event Custom|OnComponentEndOverlap_Event
  (params (OverlappedComponent :type Primitive%20Component%20Object%20Reference) (OtherActor :type Actor%20Object%20Reference) (OtherComp :type Primitive%20Component%20Object%20Reference) (OtherBodyIndex :type Integer))
  ;[1 1 1] Character Possession Code, and yah it is fucking to long . . . BUT IT WORKS
  (Variables|Default|SetOverlap%20Bool false)
  (Development|PrintString "NOT"))

(event Custom|Reset-2
  ;[1 1 1] Character Possession Code, and yah it is fucking to long . . . BUT IT WORKS
  (Utilities|FlowControl|DoOnce false) ; enters at Reset
)

(event Custom|TurborlaserOverlap
  (bind _returnvalue (Pawn|GetControlledPawn))
  (bind _firstpersoncharacter (Variables|Default|GetFirstPersonCharacter))
  (bind _returnvalue_2 (Utilities|GetClass _returnvalue))
  (bind _spherecomponent (Variables|/Game/Blueprints/Characters/Character_Base.Character_Base_C|GetSphereComponent _firstpersoncharacter))
  ;[1 1 1] Character Possession Code, and yah it is fucking to long . . . BUT IT WORKS
  (Utilities|FlowControl|Sequence
    (:then_0
      (Variables|Default|SetIs%20TurboLaser (== _returnvalue_2 "/Game/Blueprints/Characters/TurboLaser.TurboLaser_C") :!label _label)
      (Variables|Default|SetIs%20Character (== _returnvalue_2 "/Game/Blueprints/Characters/Character_Base.Character_Base_C")))
    (:then_1
      (if (Variables|Default|GetIs%20AiReady)
        (Utilities|FlowControl|Sequence
          (:then_0
            (Collision|BindEventtoOnComponentBeginOverlap _spherecomponent (delegate Custom|OnComponentBeginOverlap_Event))
            (goto _label))
          (:then_1
            (Collision|BindEventtoOnComponentEndOverlap _spherecomponent (delegate Custom|OnComponentEndOverlap_Event))))))))

(event Custom|CaptureZoneOverlap
  ;[1 1 1] Character Possession Code, and yah it is fucking to long . . . BUT IT WORKS
)

(event Custom|OnComponentBeginOverlap_Event
  (params (OverlappedComponent :type Primitive%20Component%20Object%20Reference) (OtherActor :type Actor%20Object%20Reference) (OtherComp :type Primitive%20Component%20Object%20Reference) (OtherBodyIndex :type Integer) (bFromSweep :type Boolean) (SweepResult :type Hit%20Result%20Structure%20%28by%20ref%29))
  ;[1 1 1] Character Possession Code, and yah it is fucking to long . . . BUT IT WORKS
  (Development|PrintString (Utilities|GetDisplayName OtherActor) false)
  (bind _asturbo_laser (Utilities|Casting|CastToTurboLaser OtherActor))
  (Variables|Default|SetPossessedTurboLaser _asturbo_laser)
  (Variables|Default|SetOverlap%20Bool true)
  (Development|PrintString "Overlapped" false))

(event EventBeginPlay
  ;[1 1 1] Character Possession Code, and yah it is fucking to long . . . BUT IT WORKS
  (Variables|Default|SetIs%20AiReady true)
  (Utilities|FlowControl|Sequence
    (:then_0
      (bind _outactors (Actor|GetAllActorsOfClass "/Game/Blueprints/Characters/TurboLaser.TurboLaser_C"))
      (for (_array_element _array_index) _outactors
        (Variables|Default|SetTurboLaser _array_element)
        (Development|PrintString (Utilities|String|ToString(Integer) _array_index))
        (bind _outactors_2 (Actor|GetAllActorsOfClass "/Game/Blueprints/Characters/Character_Base.Character_Base_C"))
        (for _array_element_2 _outactors_2
          (Variables|Default|SetFirstPersonCharacter _array_element_2)
          (Development|PrintString (Utilities|GetDisplayName (Pawn|GetControlledPawn))))))))

(event EventTick
  (params (DeltaSeconds :type Float%20%28single-precision%29))
  (CallFunction|TurborlaserOverlap))

(event Input|KeyboardEvents|E
  (params (Key :type Key%20Structure))
  ;[1 1 1] Character Possession Code, and yah it is fucking to long . . . BUT IT WORKS
  (:Pressed
    (Utilities|FlowControl|Sequence
      (:then_0
        (if (Variables|Default|GetIs%20Character)
          (if (Variables|Default|GetOverlap%20Bool)
            (Utilities|FlowControl|DoOnce false
              (:Completed
                (Pawn|Possess (Game|GetPlayerController 0) (stale Custom|OnComponentBeginOverlap_Event _asturbo_laser))
                (Actor|DestroyActor (Variables|Default|GetFirstPersonCharacter))
                (Variables|Default|SetIs%20AiReady false)
                (CallFunction|Reset-1))))))
      (:then_1
        (if (Variables|Default|GetIs%20TurboLaser)
          (Utilities|FlowControl|DoOnce false
            (:Completed
              (bind _returnvalue (Game|SpawnActorfromClass "/Game/Blueprints/Characters/Character_Base.Character_Base_C" (Math|Transform|MakeTransform (+ (.Location (Math|Transform|BreakTransform (Transformation|GetWorldTransform (Variables|/Game/Blueprints/Characters/TurboLaser.TurboLaser_C|GetCamera (Variables|Default|GetTurboLaser))))) "100.000000, 0,1000.000000")) "Undefined" 0 0))
              (Pawn|Possess (Game|GetPlayerController 0) _returnvalue)
              (Variables|Default|SetIs%20AiReady true)
              (CallFunction|Reset-2)))))
      (:then_2
        (Utilities|FlowControl|Sequence
          (:then_0
            (bind _outactors (Actor|GetAllActorsOfClass "/Game/Blueprints/Characters/TurboLaser.TurboLaser_C"))
            (for (_array_element _array_index) _outactors
              (Variables|Default|SetTurboLaser _array_element)
              (Development|PrintString (Utilities|String|ToString(Integer) _array_index))
              (bind _outactors_2 (Actor|GetAllActorsOfClass "/Game/Blueprints/Characters/Character_Base.Character_Base_C"))
              (for _array_element_2 _outactors_2
                (Variables|Default|SetFirstPersonCharacter _array_element_2)
                (Development|PrintString (Utilities|GetDisplayName (Pawn|GetControlledPawn)))))))))))

(fn ConstructionScript)