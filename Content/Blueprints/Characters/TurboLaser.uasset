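; TurboLaser is a turret that a player aims and fires, while unpossessed turrets track the player.
; Turn and LookUp input rotate the Arrow, and a Tick-polled gate opened by Fire input spawns Lasers with sound from two muzzle arrows.
; On the server, Tick rotates the other TurboLasers toward player zero, excluding the controller's possessed one.
; AI firing is an empty stub, and F toggles a temporary third-person camera.
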(event Custom|Fire
  ;[1 1 1] LONGEST PIECE OF SHIT CODE FOR FIRING A GUN!!!
  (Utilities|FlowControl|Gate true
    (:Exit
      (|ForEachEButtonPressMethod
        (:LoopBody
          (Utilities|FlowControl|Delay 0.2)
          (Utilities|FlowControl|Sequence
            (:then_0
              (bind _transform (Utilities|FuckNugget (Variables|Default|GetArrow1)))
              (Game|SpawnActorfromClass "/Game/Blueprints/Characters/Laser.Laser_C" _transform "AlwaysSpawn" 0 0) ; Spawn projectile
              (Audio|PlaySoundatLocation "/Game/FirstPerson/Audio/FirstPersonTemplateWeaponFire02.FirstPersonTemplateWeaponFire02" (Transformation|GetActorLocation)) ; Play firing sound
            )
            (:then_1
              (bind _transform_2 (Utilities|FuckNugget (Variables|Default|GetArrow2)))
              (Game|SpawnActorfromClass "/Game/Blueprints/Characters/Laser.Laser_C" _transform_2 "AlwaysSpawn" 0 0) ; Spawn projectile
              (Audio|PlaySoundatLocation "/Game/FirstPerson/Audio/FirstPersonTemplateWeaponFire02.FirstPersonTemplateWeaponFire02" (Transformation|GetActorLocation)) ; Play firing sound
            )))))))

(event Custom|AiMovement
  ;[1 1 1] AiTurretMovementSystem
  (Networking|SwitchHasAuthority
    (:Authority
      (Utilities|Array|RemoveItem (Variables|Default|GetAllTurboLasers) (Variables|/Game/Blueprints/GamePlay/MainCharacterController.MainCharacterController_C|GetPossessedTurboLaser (Variables|Default|GetMainCharacterController)))
      (for _array_element (Variables|Default|GetAllTurboLasers)
        (CallFunction|RotateMeshtoTargetActor (Variables|TurboLaser_C|GetArrow _array_element) (Game|Player|GetPlayerPawn 0) (Variables|Default|GetDeltaTime) 1e+01 -1.0 9e+01 false false)))))

(event Custom|AiFire
  (params (EnemyDetected :type Boolean) (AiReady :type Boolean))
  ;[1 1 1] LONGEST PIECE OF SHIT CODE FOR FIRING A GUN!!!
)

(event EventBeginPlay
  ;[1 1 1] BeginPlayUpdates
  (bind _outactors (Actor|GetAllActorsOfClass "/Game/Blueprints/GamePlay/MainCharacterController.MainCharacterController_C"))
  (for _array_element _outactors
    (Variables|Default|SetMainCharacterController _array_element)
    (bind _outactors_2 (Actor|GetAllActorsOfClass "TurboLaser_C"))
    (Variables|Default|SetAllTurboLasers _outactors_2)))

(event EventTick
  (params (DeltaSeconds :type Float%20%28single-precision%29))
  ;[1 1 1] Event Tick Updates
  (Variables|Default|SetDeltaTime DeltaSeconds)
  (CallFunction|Fire)
  (CallFunction|AiFire false false)
  (CallFunction|AiMovement))

(event Input|ActionEvents|InputActionFire
  (params (Key :type Key%20Structure))
  ;[1 1 1] LONGEST PIECE OF SHIT CODE FOR FIRING A GUN!!!
  (:Pressed
    (Utilities|FlowControl|Gate true) ; enters at Open
  )
  (:Released
    (Utilities|FlowControl|Gate true) ; enters at Close
  ))

(event Input|AxisEvents|InputAxisLookUp
  (params (AxisValue :type Float%20%28single-precision%29))
  (bind _arrow (Variables|Default|GetArrow))
  ;[1 1 1] PlayerTurretMovementSystem
  (Transformation|SetWorldRotation _arrow (Utilities|LocationofStaticMesh _arrow AxisValue 0.0 0.0) false false))

(event Input|AxisEvents|InputAxisTurn
  (params (AxisValue :type Float%20%28single-precision%29))
  (bind _arrow (Variables|Default|GetArrow))
  ;[1 1 1] PlayerTurretMovementSystem
  (Transformation|SetWorldRotation _arrow (Utilities|LocationofStaticMesh _arrow 0.0 0.0 AxisValue) false false))

(event Input|KeyboardEvents|F
  (params (Key :type Key%20Structure))
  ;[1 1 1] Temp 3rd Person Mode
  (:Pressed
    (Utilities|FlowControl|FlipFlop
      (:A
        (Components|Activation|Deactivate (Variables|Default|GetCamera))
        (Components|Activation|Activate (Variables|Default|GetCamera1) false))
      (:B
        (Components|Activation|Deactivate (Variables|Default|GetCamera1))
        (Components|Activation|Activate (Variables|Default|GetCamera) false)))))

(fn ConstructionScript)

(fn RotateAround
  (params (Center :type Vector) (Rotation :type Rotator) (Distance :type Float%20%28single-precision%29))
  (bind _returnvalue (Math|Vector|GetForwardVector Rotation))
  (bind _returnvalue_2 (* _returnvalue Distance))
  (bind _returnvalue_3 (+ Center _returnvalue_2))
  (bind (_x _y _z) (Math|Vector|BreakVector _returnvalue_3))
  (return "0, 0, 0" (Math|Rotator|MakeRotator _x _y _z)))

(fn OnRepMainCharacterController)