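; Blueprint function library with helpers for aiming a mesh at a target actor and checking the target's distance.
; RotateMeshToTargetActor uses RInterpTo toward a look-at rotation, remapping scaled pitch into roll, offsetting yaw and zeroing pitch.
; TargetNearBy returns at-or-below and at-or-above threshold booleans, using GetPointDistanceToLine with a zero direction as a point-to-point distance from the mesh.
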(fn RotateMeshtoTargetActor
  (params (MeshToRotate :type Scene%20Component%20Object%20Reference) (Target :type Actor%20Object%20Reference) (DeltaTime :type Float%20%28single-precision%29) (InterpSpeed :type Float%20%28single-precision%29) (Y%20*%20F :type Float%20%28single-precision%29) (Z%20-%20F :type Float%20%28single-precision%29) (bSweep :type Boolean) (bTeleport :type Boolean))
  (bind _returnvalue (Transformation|GetWorldLocation MeshToRotate))
  (bind _returnvalue_2 (Transformation|GetActorLocation Target))
  (bind _returnvalue_3 (Math|Rotator|FindLookatRotation _returnvalue _returnvalue_2))
  (bind (_roll _pitch _yaw) (Math|Rotator|BreakRotator _returnvalue_3))
  (bind _sweephitresult (Transformation|SetWorldRotation MeshToRotate (Math|Interpolation|RInterpTo (Transformation|GetWorldRotation MeshToRotate) (Math|Rotator|MakeRotator (* _pitch Y%20*%20F) 0.0 (- _yaw Z%20-%20F)) DeltaTime InterpSpeed) bSweep bTeleport))
  (return _sweephitresult))

(fn TargetNearby
  (params (Target :type Actor%20Object%20Reference) (Mesh :type Scene%20Component%20Object%20Reference) (Value%20<=A :type Float%20%28single-precision%29) (Value%20>=A :type Float%20%28single-precision%29))
  (bind _returnvalue (Transformation|GetActorLocation Target))
  (bind _returnvalue_2 (Transformation|GetWorldLocation Mesh))
  (bind _returnvalue_3 (Math|Vector|GetPointDistancetoLine _returnvalue _returnvalue_2 "0, 0, 0"))
  (return (<= _returnvalue_3 Value%20<=A) (>= _returnvalue_3 Value%20>=A)))