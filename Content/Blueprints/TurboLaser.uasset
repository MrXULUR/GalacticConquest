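; TurboLaser is a player-controlled twin laser turret, with Turn and LookUp input feeding the Arrow's world rotation and F toggling between two cameras.
; Holding Fire runs a delayed loop that spawns Laser actors with sound at Sphere and Sphere1, using zero rotation, until release.
; A Pawn Rotation macro that eases the Barrel's yaw toward the player is defined but not called in the event graph.
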(event EventTick
  (params (DeltaSeconds :type Float%20%28single-precision%29))
  ;[1 1 1] Event Tick Updates
  (Variables|Default|SetDeltaTime DeltaSeconds))

(event Input|ActionEvents|InputActionFire
  (params (Key :type Key%20Structure))
  (:Pressed
    (Variables|Default|SetIsReleased false)
    (|ForEachEButtonPressMethod :!label _label
      (:LoopBody
        (Utilities|FlowControl|Delay 0.2)
        (Utilities|FlowControl|Sequence
          (:then_0
            (bind _transform (Utilities|NewMacro0 (Variables|Default|GetGunOffset) 0 0 (Variables|Default|GetSphere)))
            (Game|SpawnActorfromClass "/Game/Blueprints/Laser.Laser_C" _transform "AlwaysSpawn" 0 0) ; Spawn projectile
            (Audio|PlaySoundatLocation "/Game/FirstPerson/Audio/FirstPersonTemplateWeaponFire02.FirstPersonTemplateWeaponFire02" (Transformation|GetActorLocation)) ; Play firing sound
          )
          (:then_1
            (bind _transform_2 (Utilities|NewMacro0 (Variables|Default|GetGunOffset) 0 0 (Variables|Default|GetSphere1)))
            (Game|SpawnActorfromClass "/Game/Blueprints/Laser.Laser_C" _transform_2 "AlwaysSpawn" 0 0) ; Spawn projectile
            (Audio|PlaySoundatLocation "/Game/FirstPerson/Audio/FirstPersonTemplateWeaponFire02.FirstPersonTemplateWeaponFire02" (Transformation|GetActorLocation)) ; Play firing sound
            (if (not (Variables|Default|GetIsReleased))
              (goto _label)))))))
  (:Released
    (Variables|Default|SetIsReleased true)))

(event Input|AxisEvents|InputAxisLookUp
  (params (AxisValue :type Float%20%28single-precision%29))
  (bind _arrow (Variables|Default|GetArrow))
  ;[1 1 1] PlayerTurretMovementSystem
  (Transformation|SetWorldRotation _arrow (Utilities|LocationofStaticMesh _arrow AxisValue 0.0 0.0) false false))

(event Input|AxisEvents|InputAxisTurn
  (params (AxisValue :type Float%20%28single-precision%29))
  (bind _arrow (Variables|Default|GetArrow))
  ;[1 1 1] PlayerTurretMovementSystem
  (Transformation|SetWorldRotation _arrow (Utilities|LocationofStaticMesh _arrow 0.0 0.0 AxisValue) false false))

(event Input|KeyboardEvents|F
  (params (Key :type Key%20Structure))
  (:Pressed
    (Utilities|FlowControl|FlipFlop
      (:A
        (Components|Activation|Deactivate (Variables|Default|GetCamera))
        (Components|Activation|Activate (Variables|Default|GetCamera1) false))
      (:B
        (Components|Activation|Deactivate (Variables|Default|GetCamera1))
        (Components|Activation|Activate (Variables|Default|GetCamera) false)))))

(fn ConstructionScript)

(fn RotateAround
  (params (Center :type Vector) (Rotation :type Rotator) (Distance :type Float%20%28single-precision%29))
  (bind _returnvalue (Math|Vector|GetForwardVector Rotation))
  (bind _returnvalue_2 (* _returnvalue Distance))
  (bind _returnvalue_3 (+ Center _returnvalue_2))
  (bind (_x _y _z) (Math|Vector|BreakVector _returnvalue_3))
  (return "" (Math|Rotator|MakeRotator _x _y _z)))